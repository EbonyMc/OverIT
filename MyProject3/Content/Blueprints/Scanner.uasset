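; Scanner Blueprint that scans Scannables actors as they leave its Box trigger, or reloads Level1 if the item's Reset flag is set.
; Scanning marks the item scanned, stores its point value and plays a barcode beep.
; If the item also casts to Spawner, its name variable picks the red or yellow scan material and the Money component activates.
; Beginning an overlap restores the neutral material.
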(event OnComponentBeginOverlap(Box)
  (params (OverlappedComponent :type Primitive%20Component%20Object%20Reference) (OtherActor :type Actor%20Object%20Reference) (OtherComp :type Primitive%20Component%20Object%20Reference) (OtherBodyIndex :type Integer) (bFromSweep :type Boolean) (SweepResult :type Hit%20Result%20Structure%20%28by%20ref%29))
  (Rendering|Material|SetMaterial (Variables|Default|GetStaticMesh) 1 "/Game/Materials/nuetral.nuetral"))

(event OnComponentEndOverlap(Box)
  (params (OverlappedComponent :type Primitive%20Component%20Object%20Reference) (OtherActor :type Actor%20Object%20Reference) (OtherComp :type Primitive%20Component%20Object%20Reference) (OtherBodyIndex :type Integer))
  ;[1 1 1] Scanning stuff
  (bind _asscannables (Utilities|Casting|CastToScannables (stale OnComponentBeginOverlap(Box) OtherActor)))
  (if (Variables|/Game/Blueprints/Scannables.Scannables_C|GetReset _asscannables)
    (Game|OpenLevel(byName) "Level1")
    (else
      (Variables|/Game/Blueprints/Scannables.Scannables_C|SetIsScanned _asscannables true)
      (Variables|Default|SetcurrentPointsValue (Variables|/Game/Blueprints/Scannables.Scannables_C|GetPointsvalue _asscannables))
      (Audio|PlaySoundatLocation "/Game/Audio/se_barcodeBeep__1_.se_barcodeBeep__1_" (Transformation|GetActorLocation _asscannables) "0, 0, 0" 1.0 1.0 0.0 0 0 0)
      (bind _asspawner (Utilities|Casting|CastToSpawner OtherActor))
      (Variables|Default|SetcurrentColor (Variables|/Game/Blueprints/Spawner.Spawner_C|GetNamehere _asspawner))
      ;[1 1 1] Color change
      (if (Utilities|Name|Equal(Name) (Variables|Default|GetcurrentColor) "Red")
        (Rendering|Material|SetMaterial (Variables|Default|GetStaticMesh) 1 "/Game/Materials/rescan.rescan")
        (else
          (Rendering|Material|SetMaterial (Variables|Default|GetStaticMesh) 1 "/Game/Materials/yellowscan.yellowscan")))
      (Components|Activation|Activate (Variables|Default|GetMoney) false))))

(fn ConstructionScript)