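; Eats is an AI-moved creature that appears once the player reaches 150 points and eats Scannables.
; Tele polls every 0.2 seconds, then teleports it to Point and sets Canmove.
; Movement, checked once five seconds after BeginPlay, loops between Point and Pont2 only if Canmove is already set.
; Scannables overlapping BoxForPoints award points; those overlapping BoxFortongue get attached to the tongue, moved by single-step VInterpTo, and destroyed.
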(event OnComponentBeginOverlap(BoxForPoints)
  (params (OverlappedComponent :type Primitive%20Component%20Object%20Reference) (OtherActor :type Actor%20Object%20Reference) (OtherComp :type Primitive%20Component%20Object%20Reference) (OtherBodyIndex :type Integer) (bFromSweep :type Boolean) (SweepResult :type Hit%20Result%20Structure%20%28by%20ref%29))
  (Utilities|Casting|CastToScannables OtherActor)
  (bind _asmotion_controller_pawn (Utilities|Casting|CastToMotionControllerPawn (Game|Player|GetPlayerPawn 0)))
  (Default|Addingpoints _asmotion_controller_pawn 5))

(event OnComponentBeginOverlap(BoxFortongue)
  (params (OverlappedComponent :type Primitive%20Component%20Object%20Reference) (OtherActor :type Actor%20Object%20Reference) (OtherComp :type Primitive%20Component%20Object%20Reference) (OtherBodyIndex :type Integer) (bFromSweep :type Boolean) (SweepResult :type Hit%20Result%20Structure%20%28by%20ref%29))
  (bind _tounge (Variables|Default|GetTounge))
  (bind _asscannables (Utilities|Casting|CastToScannables OtherActor))
  (Variables|Default|SetScannables _asscannables)
  (Rendering|SetVisibility (Variables|Default|GetTounge) true false)
  (Transformation|SetWorldLocation _tounge (Math|Interpolation|VInterpTo (Transformation|GetWorldLocation (Variables|Default|GetBoxForPoints)) (Transformation|GetActorLocation _asscannables) 2.0 5.0) false false)
  (Transformation|AttachComponentToComponent (Variables|Default|GetScannables) _tounge "None" "SnapToTarget" "SnapToTarget" "KeepWorld" true)
  (Utilities|FlowControl|Delay 0.2)
  (Transformation|SetWorldLocation (Variables|Default|GetTounge) (Math|Interpolation|VInterpTo (Transformation|GetActorLocation (Variables|Default|GetScannables)) (Transformation|GetWorldLocation (Variables|Default|GetBoxForPoints)) 2.0 5.0) false false)
  (Actor|DestroyActor (Variables|Default|GetScannables))
  (Rendering|SetVisibility (Variables|Default|GetTounge) false false))

(event Custom|Movement
  (if (Variables|Default|GetCanmove)
    (AI|AIMoveTo self "0, 0, 0" (Variables|Default|GetPoint) 2.0 false
      (:then
        (Utilities|FlowControl|Delay 5.0)
        (AI|AIMoveTo self "0, 0, 0" (Variables|Default|GetPont2) 2.0 false
          (:then
            (Utilities|FlowControl|Delay 5.0)
            (CallFunction|Movement)))))))

(event Custom|Tele
  (bind _asmotion_controller_pawn (Utilities|Casting|CastToMotionControllerPawn (Game|Player|GetPlayerPawn 0) :!label _label))
  (if (>= (Variables|/Game/VirtualRealityBP/Blueprints/MotionControllerPawn.MotionControllerPawn_C|GetPoints _asmotion_controller_pawn) 150)
    (Transformation|SetActorLocation (Transformation|GetActorLocation (Variables|Default|GetPoint)) false true)
    (Variables|Default|SetCanmove true)
    (else
      (Utilities|FlowControl|Delay 0.2)
      (goto _label))))

(event EventBeginPlay
  (CallFunction|Tele)
  (Utilities|Time|SetTimerbyFunctionName 0 "Movement" 5.0))

(fn ConstructionScript)