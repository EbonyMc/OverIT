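; Truck Blueprint that moves along a referenced spline, with movement scaled by an axis value.
; Addmovement advances the distance along the spline by speed, axis value and delta time.
; UpdatelocationandRotation samples the spline at that distance, applying its X, Y and rotation while keeping the truck's current Z.
; The event graph does not call either function, and BeginPlay only assigns Walkspeed to itself.
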(event EventBeginPlay
  (Variables|Default|SetWalkspeed (Variables|Default|GetWalkspeed)))

(fn ConstructionScript)

(fn UpdatelocationandRotation
  (bind _splineref (Variables|Default|GetSplineref))
  (bind _distancealongspline (Variables|Default|GetDistancealongspline))
  (bind _spline (Variables|/Game/Blueprints/Truckfollowspline/Splineline.Splineline_C|GetSpline _splineref))
  (bind _returnvalue (Spline|GetLocationatDistanceAlongSpline _spline _distancealongspline "World"))
  (Transformation|SetActorLocationAndRotation (Math|Vector|MakeVector (.x _returnvalue) (.y _returnvalue) (.z (Transformation|GetActorLocation))) (Spline|GetRotationatDistanceAlongSpline _spline (Variables|Default|GetDistancealongspline) "World")))

(fn Addmovement
  (bind _speed (Variables|Default|GetSpeed))
  (bind _axis_value (Variables|Default|GetAxis%20Value))
  (bind _returnvalue (* _speed _axis_value))
  (Variables|Default|SetAcel _returnvalue)
  (Variables|Default|SetDistancealongspline (+ (Variables|Default|GetDistancealongspline) (* _returnvalue (Utilities|Time|GetWorldDeltaSeconds)))))