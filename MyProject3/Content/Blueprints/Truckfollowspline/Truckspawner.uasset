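; Truck spawner actor that fills every Splineline in the level with AI trucks on BeginPlay.
; For each spline it spaces that spline's set number of trucks evenly along its length, cycling through the spline's array of truck classes.
; Each truck gets its spline reference and starting distance, then a default controller.
; The class index carries over between splines, while the distance resets.
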(event EventBeginPlay
  (bind _outactors (Actor|GetAllActorsOfClass "/Game/Blueprints/Truckfollowspline/Splineline.Splineline_C"))
  (Variables|Default|SetSplineref _outactors)
  (CallFunction|SpawnnextSpline))

(fn ConstructionScript)

(fn SpawnnextSpline
  ;[1 1 1] calculates how many characters on the spline based on the number of characters on spline var
  (for _array_element (Variables|Default|GetSplineref)
    (bind _output_get (LocalVariables|SetcurrentSpline _array_element))
    (LocalVariables|SetSplineDivision (/ (Spline|GetSplineLength (Variables|/Game/Blueprints/Truckfollowspline/Splineline.Splineline_C|GetSpline _output_get)) (Math|Conversions|ToFloat(Integer) (Variables|/Game/Blueprints/Truckfollowspline/Splineline.Splineline_C|Getnumberoftrucksonspline _output_get))))
    (for _index (range 1 (Variables|/Game/Blueprints/Truckfollowspline/Splineline.Splineline_C|Getnumberoftrucksonspline _output_get))
      ;[1 1 1] spawncharacter based on the current distance
      (bind _returnvalue (Game|SpawnActorfromClass (Utilities|Array|Get(acopy) (Variables|/Game/Blueprints/Truckfollowspline/Splineline.Splineline_C|GetAmmountoftrucks (LocalVariables|GetcurrentSpline)) (LocalVariables|GetSplinecharindex)) (Math|Transform|MakeTransform (Spline|GetLocationatDistanceAlongSpline (Variables|/Game/Blueprints/Truckfollowspline/Splineline.Splineline_C|GetSpline (LocalVariables|GetcurrentSpline)) (LocalVariables|GetCurdist) "World") (Spline|GetRotationatDistanceAlongSpline (Variables|/Game/Blueprints/Truckfollowspline/Splineline.Splineline_C|GetSpline (LocalVariables|GetcurrentSpline)) (LocalVariables|GetCurdist) "World") "1,1.000000,1") "AdjustIfPossibleButAlwaysSpawn" 0 0))
      ;[1 1 1] Set character varables and spawn ai controls
      (Variables|/Game/Blueprints/Truckfollowspline/truck.truck_C|SetSplineref _returnvalue (LocalVariables|GetcurrentSpline))
      (Variables|/Game/Blueprints/Truckfollowspline/truck.truck_C|SetDistancealongspline _returnvalue (LocalVariables|GetCurdist))
      (Pawn|SpawnDefaultController _returnvalue)
      ;[1 1 1] updated distance alongspline
      (LocalVariables|SetCurdist (+ (LocalVariables|GetCurdist) (LocalVariables|GetSplineDivision)))
      (if (>= (LocalVariables|GetSplinecharindex) (- (Utilities|Array|Length (Variables|/Game/Blueprints/Truckfollowspline/Splineline.Splineline_C|GetAmmountoftrucks (LocalVariables|GetcurrentSpline))) 1))
        (LocalVariables|SetSplinecharindex 0)
        (else
          (Math|Integer|IncrementInt (LocalVariables|GetSplinecharindex)))))
    (LocalVariables|SetCurdist 0.0)))