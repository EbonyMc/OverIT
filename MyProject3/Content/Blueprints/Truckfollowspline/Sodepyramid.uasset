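; Sodepyramid is a soda prop actor, likely one piece of a pyramid, that tumbles under physics and later resets.
; On BeginPlay it saves the Sodar component's transform and keeps its physics off.
; A Scannables actor overlapping its Box calls Setphysic on every Sodepyramid in the level.
; Setphysic enables physics, waits on a delay, restores the saved transform, disables physics, then adds an impulse while simulation is off.
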(event OnComponentBeginOverlap(Box)
  (params (OverlappedComponent :type Primitive%20Component%20Object%20Reference) (OtherActor :type Actor%20Object%20Reference) (OtherComp :type Primitive%20Component%20Object%20Reference) (OtherBodyIndex :type Integer) (bFromSweep :type Boolean) (SweepResult :type Hit%20Result%20Structure%20%28by%20ref%29))
  ;[1 1 1] Detects the scannable and activate physic
  (Utilities|Casting|CastToScannables OtherActor)
  (bind _outactors (Actor|GetAllActorsOfClass "Sodepyramid_C"))
  (for _array_element _outactors
    (CallFunction|Setphysic _array_element)))

(event Custom|Setphysic
  (bind _sodar (Variables|Default|GetSodar))
  ;[1 1 1] Set physics in motion then resets the postion and makes it back to floating
  (Physics|SetSimulatePhysics _sodar true)
  (Utilities|FlowControl|Delay 2e+01)
  (Transformation|SetWorldTransform _sodar (Variables|Default|GetSavespot) false false)
  (Physics|SetSimulatePhysics (Variables|Default|GetSodar) false)
  (Physics|AddImpulse (Variables|Default|GetSodar) "0,9000.000000,9000.000000" "None" false))

(event EventBeginPlay
  (bind _sodar (Variables|Default|GetSodar))
  ;[1 1 1] set objects
  (Variables|Default|SetSoda _sodar)
  (Variables|Default|SetSavespot (Transformation|GetWorldTransform _sodar))
  (Physics|SetSimulatePhysics (Variables|Default|GetSodar) false))

(fn ConstructionScript)