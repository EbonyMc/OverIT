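; Truck Blueprint that moves along a referenced spline in a continuous loop.
; Each tick it calls Addmovement, then UpdatelocationandRotation to handle movement, position and orientation.
; When the distance along the spline comes within a small tolerance of the spline's length, it resets to zero to restart the route.
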(event EventBeginPlay
  (|CallParentFunction))

(event EventTick
  (params (DeltaSeconds :type Float%20%28single-precision%29))
  ;[1 1 1] set the rotation and movement
  (CallFunction|Addmovement)
  (CallFunction|UpdatelocationandRotation)
  ;[1 1 1] reset when reaching the end of the spline
  (if (Math|Float|NearlyEqual(Float) (Variables|Default|GetDistancealongspline) (Spline|GetSplineLength (Variables|/Game/Blueprints/Truckfollowspline/Splineline.Splineline_C|GetSpline (Variables|Default|GetSplineref))) 1e+01)
    (Variables|Default|SetDistancealongspline 0.0)))

(fn ConstructionScript
  (|CallParentFunction))