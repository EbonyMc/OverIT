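; Spawner that creates random scannable items at TargetPoints for a game using a MotionControllerPawn.
; A timer spawns items unless the last found one is floating, then sphere-traces between the first two TargetPoints to give the hit Scannables a random mesh, material, color name, points and sometimes a special behavior or sound.
; A second timer widens the item pool as player Points pass rising thresholds.
; Detect and the timeline movement are unused.
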(event Custom|SpawnItem
  (bind _scanables (Variables|Default|GetScanables))
  (if (not (Variables|/Game/Blueprints/Scannables.Scannables_C|GetIsFloating (Variables|Default|GetScanVar)))
    (bind _outactors (Actor|GetAllActorsOfClass "/Script/Engine.TargetPoint"))
    ;[1 1 1] Teleport objects to specific points
    (Game|SpawnActorfromClass (Utilities|Array|Get(acopy) _scanables (Math|Random|RandomInteger (Utilities|Array|Length _scanables))) (Math|Transform|MakeTransform (Transformation|GetActorLocation (Utilities|Array|Get(acopy) _outactors (Math|Random|RandomInteger (Utilities|Array|Length _outactors)))) (Transformation|GetActorRotation (Utilities|Array|Get(acopy) _outactors (Math|Random|RandomInteger (Utilities|Array|Length _outactors)))) "1.200000,1.200000,1.200000") "Undefined" 0 0)
    (CallFunction|TransferObject)))

(event Custom|TransferObject
  ;[1 1 1] Transfer object points and mesh
  (bind (_outhit _returnvalue) (Collision|SphereTraceByChannel (Transformation|GetActorLocation (Utilities|Array|Get(acopy) (stale Custom|SpawnItem _outactors))) (Transformation|GetActorLocation (Utilities|Array|Get(acopy) (stale Custom|SpawnItem _outactors) 1)) 5e+01 "TraceTypeQuery3" false 0 "None"))
  (if _returnvalue
    (bind _asscannables (Utilities|Casting|CastToScannables (.HitActor (Collision|BreakHitResult _outhit))))
    (Variables|Default|SetScanVar _asscannables)
    (Variables|/Game/Blueprints/Scannables.Scannables_C|SetKill _asscannables false)
    (switch int (Math|Integer|Clamp(Integer) (Math|Random|RandomIntegerinRange 0 (Variables|Default|GetItems)) 0 14)
      (:0
        (bind _output_get (Variables|Default|SetNamehere "Red" :!label _label))
        ;;[1 1 1] Milk
        (Variables|/Game/Blueprints/Scannables.Scannables_C|SetThisWillChange (Variables|Default|GetScanVar) _output_get)
        (Components|StaticMesh|SetStaticMesh (Variables|/Script/Engine.StaticMeshActor|GetStaticMeshComponent (Variables|Default|GetScanVar)) "/Game/Geometry/Objects/hs_sack.hs_sack")
        (Rendering|Material|SetMaterial (Variables|/Script/Engine.StaticMeshActor|GetStaticMeshComponent (Variables|Default|GetScanVar)) 0 "/Game/Materials/hs_sack_Mat.hs_sack_Mat")
        (Variables|/Game/Blueprints/Scannables.Scannables_C|SetPointsvalue (Variables|Default|GetScanVar) 5))
      (:1
        (goto _label))
      (:2
        (bind _output_get_2 (Variables|Default|SetNamehere "Red" :!label _label_2))
        (Variables|/Game/Blueprints/Scannables.Scannables_C|SetThisWillChange (Variables|Default|GetScanVar) _output_get_2)
        ;[1 1 1] Soda
        (Components|StaticMesh|SetStaticMesh (Variables|/Script/Engine.StaticMeshActor|GetStaticMeshComponent (Variables|Default|GetScanVar)) "/Game/Geometry/Objects/hs_soda.hs_soda")
        (Rendering|Material|SetMaterial (Variables|/Script/Engine.StaticMeshActor|GetStaticMeshComponent (Variables|Default|GetScanVar)) 0 "/Game/Materials/hs_soda.hs_soda")
        (Variables|/Game/Blueprints/Scannables.Scannables_C|SetPointsvalue (Variables|Default|GetScanVar) 10))
      (:3
        (goto _label_2))
      (:4
        ;[1 1 1] Pack
        (bind _output_get_3 (Variables|Default|SetNamehere "Yellow" :!label _label_3))
        (Variables|/Game/Blueprints/Scannables.Scannables_C|SetThisWillChange (Variables|Default|GetScanVar) _output_get_3)
        (Components|StaticMesh|SetStaticMesh (Variables|/Script/Engine.StaticMeshActor|GetStaticMeshComponent (Variables|Default|GetScanVar)) "/Game/Geometry/Objects/hs_pack.hs_pack")
        (Rendering|Material|SetMaterial (Variables|/Script/Engine.StaticMeshActor|GetStaticMeshComponent (Variables|Default|GetScanVar)) 0 "/Game/Materials/pack_Mat.pack_Mat")
        (Variables|/Game/Blueprints/Scannables.Scannables_C|SetPointsvalue (Variables|Default|GetScanVar) 10))
      (:5
        (goto _label_3))
      (:6
        ;[1 1 1] Game
        (bind _output_get_4 (Variables|Default|SetNamehere "Yellow"))
        (Variables|/Game/Blueprints/Scannables.Scannables_C|SetThisWillChange (Variables|Default|GetScanVar) _output_get_4)
        (Components|StaticMesh|SetStaticMesh (Variables|/Script/Engine.StaticMeshActor|GetStaticMeshComponent (Variables|Default|GetScanVar)) "/Game/Geometry/Objects/hs_AlienGame.hs_AlienGame")
        (Rendering|Material|SetMaterial (Variables|/Script/Engine.StaticMeshActor|GetStaticMeshComponent (Variables|Default|GetScanVar)) 0 "/Game/Materials/mat_game.mat_game")
        (Variables|/Game/Blueprints/Scannables.Scannables_C|SetPointsvalue (Variables|Default|GetScanVar) 10)
        (Audio|PlaySound2D "/Game/Audio/Explosion_8_Bit.Explosion_8_Bit" 1.0 1.0 0.0 0 0))
      (:7
        ;[1 1 1] Cake
        (bind _output_get_5 (Variables|Default|SetNamehere "Red"))
        (Variables|/Game/Blueprints/Scannables.Scannables_C|SetThisWillChange (Variables|Default|GetScanVar) _output_get_5)
        (Components|StaticMesh|SetStaticMesh (Variables|/Script/Engine.StaticMeshActor|GetStaticMeshComponent (Variables|Default|GetScanVar)) "/Game/Geometry/Objects/hs_soda.hs_soda")
        (Rendering|Material|SetMaterial (Variables|/Script/Engine.StaticMeshActor|GetStaticMeshComponent (Variables|Default|GetScanVar)) 0 "/Game/Materials/hs_soda.hs_soda")
        (Variables|/Game/Blueprints/Scannables.Scannables_C|SetPointsvalue (Variables|Default|GetScanVar) 10))
      (:8
        ;[1 1 1] Turns to bomb
        (bind _output_get_6 (Variables|Default|SetNamehere "Yellow"))
        (Variables|/Game/Blueprints/Scannables.Scannables_C|SetThisWillChange (Variables|Default|GetScanVar) _output_get_6)
        (Default|Explode (Variables|Default|GetScanVar))
        (Components|StaticMesh|SetStaticMesh (Variables|/Script/Engine.StaticMeshActor|GetStaticMeshComponent (Variables|Default|GetScanVar)) "/Game/Geometry/Objects/hs_alienBomb.hs_alienBomb")
        (Rendering|Material|SetMaterial (Variables|/Script/Engine.StaticMeshActor|GetStaticMeshComponent (Variables|Default|GetScanVar)) 0 "/Game/Materials/hs_alienBombTexture_Mat.hs_alienBombTexture_Mat")
        (Variables|/Game/Blueprints/Scannables.Scannables_C|SetPointsvalue (Variables|Default|GetScanVar) 20))
      (:9
        ;[1 1 1] Fireworks
        (bind _output_get_7 (Variables|Default|SetNamehere "Red"))
        (Variables|/Game/Blueprints/Scannables.Scannables_C|SetThisWillChange (Variables|Default|GetScanVar) _output_get_7)
        (Default|Firework (Variables|Default|GetScanVar))
        (Components|StaticMesh|SetStaticMesh (Variables|/Script/Engine.StaticMeshActor|GetStaticMeshComponent (Variables|Default|GetScanVar)) "/Game/Geometry/Objects/hs_fireworks.hs_fireworks")
        (Rendering|Material|SetMaterial (Variables|/Script/Engine.StaticMeshActor|GetStaticMeshComponent (Variables|Default|GetScanVar)) 0 "/Game/Materials/FireWorks.FireWorks")
        (Variables|/Game/Blueprints/Scannables.Scannables_C|SetPointsvalue (Variables|Default|GetScanVar) 10))
      (:10
        ;[1 1 1] Udder
        (bind _output_get_8 (Variables|Default|SetNamehere "Yellow"))
        (Variables|/Game/Blueprints/Scannables.Scannables_C|SetThisWillChange (Variables|Default|GetScanVar) _output_get_8)
        (Components|StaticMesh|SetStaticMesh (Variables|/Script/Engine.StaticMeshActor|GetStaticMeshComponent (Variables|Default|GetScanVar)) "/Game/Geometry/Objects/hs_udder.hs_udder")
        (Rendering|Material|SetMaterial (Variables|/Script/Engine.StaticMeshActor|GetStaticMeshComponent (Variables|Default|GetScanVar)) 0 "/Game/Materials/Mat_Udder.Mat_Udder")
        (Variables|/Game/Blueprints/Scannables.Scannables_C|SetPointsvalue (Variables|Default|GetScanVar) 10)
        (Audio|PlaySound2D "/Game/Audio/Meat_Slap_2_by_mwlandi.Meat_Slap_2_by_mwlandi" 1.0 1.0 0.0 0 0))
      (:11
        ;[1 1 1] Diamond
        (bind _output_get_9 (Variables|Default|SetNamehere "Red"))
        (Variables|/Game/Blueprints/Scannables.Scannables_C|SetThisWillChange (Variables|Default|GetScanVar) _output_get_9)
        (Components|StaticMesh|SetStaticMesh (Variables|/Script/Engine.StaticMeshActor|GetStaticMeshComponent (Variables|Default|GetScanVar)) "/Game/Geometry/Objects/hs_diamond.hs_diamond")
        (Rendering|Material|SetMaterial (Variables|/Script/Engine.StaticMeshActor|GetStaticMeshComponent (Variables|Default|GetScanVar)) 0 "/Game/Materials/hs_diamond.hs_diamond")
        (Variables|/Game/Blueprints/Scannables.Scannables_C|SetPointsvalue (Variables|Default|GetScanVar) 1))
      (:12
        ;[1 1 1] Hoppers
        (bind _output_get_10 (Variables|Default|SetNamehere "Yellow"))
        (Variables|/Game/Blueprints/Scannables.Scannables_C|SetThisWillChange (Variables|Default|GetScanVar) _output_get_10)
        (Default|Hopper (Variables|Default|GetScanVar))
        (Components|StaticMesh|SetStaticMesh (Variables|/Script/Engine.StaticMeshActor|GetStaticMeshComponent (Variables|Default|GetScanVar)) "/Game/Geometry/Objects/hs_leg.hs_leg")
        (Rendering|Material|SetMaterial (Variables|/Script/Engine.StaticMeshActor|GetStaticMeshComponent (Variables|Default|GetScanVar)) 0 "/Game/Materials/hs_froggyLeg.hs_froggyLeg")
        (Variables|/Game/Blueprints/Scannables.Scannables_C|SetPointsvalue (Variables|Default|GetScanVar) 10))
      (:13
        ;[1 1 1] Vase
        (bind _output_get_11 (Variables|Default|SetNamehere "Yellow"))
        (Variables|/Game/Blueprints/Scannables.Scannables_C|SetThisWillChange (Variables|Default|GetScanVar) _output_get_11)
        (Components|StaticMesh|SetStaticMesh (Variables|/Script/Engine.StaticMeshActor|GetStaticMeshComponent (Variables|Default|GetScanVar)) "/Game/Geometry/Objects/hs_vase.hs_vase")
        (Rendering|Material|SetMaterial (Variables|/Script/Engine.StaticMeshActor|GetStaticMeshComponent (Variables|Default|GetScanVar)) 0 "/Game/Materials/mat_vase.mat_vase")
        (Variables|/Game/Blueprints/Scannables.Scannables_C|SetPointsvalue (Variables|Default|GetScanVar) 10))
      (:14
        ;[1 1 1] BoomBox
        (bind _output_get_12 (Variables|Default|SetNamehere "Yellow"))
        (Variables|/Game/Blueprints/Scannables.Scannables_C|SetThisWillChange (Variables|Default|GetScanVar) _output_get_12)
        (Components|StaticMesh|SetStaticMesh (Variables|/Script/Engine.StaticMeshActor|GetStaticMeshComponent (Variables|Default|GetScanVar)) "/Game/Geometry/Objects/hs_boombox.hs_boombox")
        (Rendering|Material|SetMaterial (Variables|/Script/Engine.StaticMeshActor|GetStaticMeshComponent (Variables|Default|GetScanVar)) 0 "/Game/Materials/hs_boombox_baseColor_Mat.hs_boombox_baseColor_Mat")
        (Variables|/Game/Blueprints/Scannables.Scannables_C|SetPointsvalue (Variables|Default|GetScanVar) 10)))))

(event Custom|Setitemcount
  ;[1 1 1] Adds one to the amountof items if a certain score is reached
  (bind _asmotion_controller_pawn (Utilities|Casting|CastToMotionControllerPawn (Game|Player|GetPlayerPawn 0)))
  (if (>= (Variables|/Game/VirtualRealityBP/Blueprints/MotionControllerPawn.MotionControllerPawn_C|GetPoints _asmotion_controller_pawn) (Variables|Default|Getitem_adder_timeset))
    (Variables|Default|SetItems (+ (Variables|Default|GetItems) 1))
    (Variables|Default|Setitem_adder_timeset (+ (Variables|Default|Getitem_adder_timeset) 15))))

(event Custom|spawn
  (Variables|Default|SetSpawnon false))

(event EventBeginPlay
  (Utilities|Time|SetTimerbyFunctionName 0 "Spawnitem" 1.0 (Variables|Default|GetSpawnon))
  (Utilities|Time|SetTimerbyFunctionName 0 "Setitemcount" 1.0 true))

(fn ConstructionScript)

(fn Detect
  ;[1 1 1] Detecting thespecfics on a object
)