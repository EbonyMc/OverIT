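; AlienSwiper is an AI-controlled alien that patrols back and forth between two placed points, Points and Point2.
; On BeginPlay it snaps to Points and starts a looping timer that calls Movement.
; A FlipFlop alternates the AI MoveToLocation target, clearing CanSwipe when heading to Point2 and setting it when returning.
; The Playanimation event is an empty stub, and several leftover nodes are disconnected.
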(event Custom|Movement
  (Utilities|FlowControl|FlipFlop
    (:A
      (AI|Navigation|MovetoLocation (AI|GetAIController self) (Transformation|GetActorLocation (Variables|Default|GetPoint2)) -1.0 true true false true 0)
      (Variables|Default|SetCanSwipe false))
    (:B
      (AI|Navigation|MovetoLocation (AI|GetAIController self) (Transformation|GetActorLocation (Variables|Default|GetPoints)) -1.0 true true false true 0)
      (Variables|Default|SetCanSwipe true))))

(event Custom|Playanimation)

(event EventBeginPlay
  (Transformation|SetActorLocation (Transformation|GetActorLocation (Variables|Default|GetPoints)) false false)
  (Utilities|Time|SetTimerbyFunctionName 0 "Movement" 3.0 true))

(fn ConstructionScript)