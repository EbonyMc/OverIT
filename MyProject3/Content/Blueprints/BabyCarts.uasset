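; Baby cart actor that loops along a referenced spline and plays reaction sounds when hit by Scannables.
; BeginPlay randomizes red or yellow material and PointsNeeded, and reveals a skeletal mesh and beam effect if the MotionControllerPawn already has enough points.
; Tick runs location and movement updates, resetting Distance near the spline's end.
; Box overlaps play a slap plus one random voice sound, throttled by a DoOnce that resets after a delay.
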(event OnComponentBeginOverlap(Box1)
  (params (OverlappedComponent :type Primitive%20Component%20Object%20Reference) (OtherActor :type Actor%20Object%20Reference) (OtherComp :type Primitive%20Component%20Object%20Reference) (OtherBodyIndex :type Integer) (bFromSweep :type Boolean) (SweepResult :type Hit%20Result%20Structure%20%28by%20ref%29))
  (Utilities|Casting|CastToScannables OtherActor)
  (Utilities|FlowControl|DoOnce false :!label _label
    (:Completed
      (Audio|PlaySound2D "/Game/Audio/Slap_Snap.Slap_Snap" 1.0 1.0 0.0 0 0)
      (switch int (Math|Random|RandomInteger 3)
        (:0
          (Audio|PlaySound2D "/Game/Audio/brrrlllack.brrrlllack" 1.0 1.0 0.0 0 0))
        (:1
          (Audio|PlaySound2D "/Game/Audio/gurgle.gurgle" 1.0 1.0 0.0 0 0))
        (:2
          (Audio|PlaySound2D "/Game/Audio/AlenYellsFreh.AlenYellsFreh" 1.0 1.0 0.0 0 0)))
      (Utilities|FlowControl|Delay 4.0)
      (goto _label Reset))))

(event EventBeginPlay
  (|CallParentFunction)
  (Utilities|FlowControl|Sequence
    (:then_0
      ;[1 1 1] Set Color
      (Variables|Default|SetNewVar_0 (Math|Random|RandomIntegerinRange 0 1))
      (if (== (Variables|Default|GetNewVar_0) 0)
        (Variables|Default|SetColor "Yellow")
        (bind _output_get (Variables|Default|SetColor2 (Utilities|Array|Get(acopy) (Variables|Default|GetMaterial))))
        (Rendering|Material|SetMaterial (Variables|Default|GetStaticMesh) 0 _output_get)
        (else
          (Variables|Default|SetColor "Red")
          (bind _output_get_2 (Variables|Default|SetColor2 (Utilities|Array|Get(acopy) (Variables|Default|GetMaterial) 1)))
          (Rendering|Material|SetMaterial (Variables|Default|GetStaticMesh) 0 _output_get_2))))
    (:then_1
      (Variables|Default|SetPointsNeeded (Math|Random|RandomIntegerinRange 10 40)))
    (:then_2
      (bind _asmotion_controller_pawn (Utilities|Casting|CastToMotionControllerPawn (Game|Player|GetPlayerPawn 0)))
      (if (>= (Variables|/Game/VirtualRealityBP/Blueprints/MotionControllerPawn.MotionControllerPawn_C|GetPoints _asmotion_controller_pawn) 50)
        (Components|Activation|Activate (Variables|Default|GetBeamy) false)
        (Rendering|SetVisibility (Variables|Default|GetSkeletalMesh) true false)))))

(event EventTick
  (params (DeltaSeconds :type Float%20%28single-precision%29))
  ;[1 1 1] Move on spline
  (CallFunction|LocationUpdate)
  (CallFunction|Movement)
  (if (Math|Float|NearlyEqual(Float) (Variables|Default|GetDistance) (Spline|GetSplineLength (Variables|/Game/Blueprints/CartSpline.CartSpline_C|GetSpline (Variables|Default|GetSplineReference))) 1e+01)
    (Variables|Default|SetDistance 0.0)))

(fn ConstructionScript
  (|CallParentFunction))