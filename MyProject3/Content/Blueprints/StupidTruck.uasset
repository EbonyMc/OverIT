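; StupidTruck is a truck actor that moves along a referenced spline in a continuous loop.
; Every tick it calls LocationUpdate and Movement, then resets Distance to zero when it comes within a small tolerance of the spline's end.
; An unconnected branch, which never runs, would randomly pick Yellow or Red and apply the matching material to the static mesh.
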(event EventBeginPlay
  (|CallParentFunction))

(event EventTick
  (params (DeltaSeconds :type Float%20%28single-precision%29))
  ;[1 1 1] Move on spline
  (CallFunction|LocationUpdate)
  (CallFunction|Movement)
  (if (Math|Float|NearlyEqual(Float) (Variables|Default|GetDistance) (Spline|GetSplineLength (Variables|/Game/Blueprints/CartSpline.CartSpline_C|GetSpline (Variables|Default|GetSplineReference))) 1e+01)
    (Variables|Default|SetDistance 0.0)))

(fn ConstructionScript
  (|CallParentFunction))