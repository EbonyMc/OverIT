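; AlienThatSwipes is an alien AI pawn that patrols back and forth between two target actors.
; On BeginPlay it starts a Movement event that uses AI Move To toward Points, waits, moves to Point2, waits, then calls itself to repeat.
; The loop continues only through each move's completion output, with failures unhandled.
; A looping timer calling Movement is present but unconnected, and no swipe logic appears.
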(event Custom|Movement
  (AI|AIMoveTo self "0, 0, 0" (Variables|Default|GetPoints) 5.0 false
    (:then
      (Utilities|FlowControl|Delay 3.0)
      (AI|AIMoveTo self "0, 0, 0" (Variables|Default|GetPoint2\) 5.0 false
        (:then
          (Utilities|FlowControl|Delay 2.0)
          (CallFunction|Movement))))))

(event EventBeginPlay
  (CallFunction|Movement))

(fn ConstructionScript)