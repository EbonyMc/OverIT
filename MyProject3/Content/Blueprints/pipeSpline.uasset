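; Pipe spline actor that builds spline mesh components along an editable spline, presumably to form a pipe.
; The construction script adds one X-forward spline mesh per point after the first and attaches it to the Scene component.
; Each mesh takes local positions and tangents from the spline, always starting at point 0 rather than the preceding point, so segments overlap instead of chaining.
; The event graph is empty.
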(event EventBeginPlay)

(event Collision|EventActorBeginOverlap
  (params (OtherActor :type Actor%20Object%20Reference)))

(event EventTick
  (params (DeltaSeconds :type Float%20%28single-precision%29)))

(fn ConstructionScript
  (bind _spline (Variables|Default|GetSpline))
  (bind (_location _tangent) (Spline|GetLocationandTangentatSplinePoint _spline 0 "Local"))
  (for _index (range 0 (- (Spline|GetNumberOfSplinePoints (Variables|Default|GetSpline)) 2))
    (bind _returnvalue (AddComponent|AddSplineMeshComponent true))
    (SplineMesh|SetForwardAxis _returnvalue "X" true)
    (Transformation|AttachComponentToComponent _returnvalue (Variables|Default|GetScene) "None" "KeepRelative" "KeepRelative" "KeepRelative" true)
    (SplineMesh|SetStartandEnd _returnvalue _location _tangent (.Location (Spline|GetLocationandTangentatSplinePoint _spline (+ _index 1) "Local")) (.Tangent (Spline|GetLocationandTangentatSplinePoint _spline (+ _index 1) "Local")) true :!class /Script/Engine.SplineMeshComponent)))