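; Alien character that wanders the navmesh holding a pen and clip, attached to mesh sockets in the construction script.
; After a short delay at BeginPlay, Movement repeatedly picks a random reachable point nearby and reissues AIMoveTo on a timed loop, without waiting for arrival.
; Capsule overlap with a Scannables actor plays an alien voice sound; its DoOnce resets only then, so any other overlap blocks later sounds.
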(event OnComponentBeginOverlap(CapsuleComponent)
  (params (OverlappedComponent :type Primitive%20Component%20Object%20Reference) (OtherActor :type Actor%20Object%20Reference) (OtherComp :type Primitive%20Component%20Object%20Reference) (OtherBodyIndex :type Integer) (bFromSweep :type Boolean) (SweepResult :type Hit%20Result%20Structure%20%28by%20ref%29))
  (Utilities|FlowControl|DoOnce false :!label _label
    (:Completed
      (Utilities|Casting|CastToScannables OtherActor)
      (Audio|PlaySoundatLocation "/Game/Audio/Alien_Voice1b.Alien_Voice1b" (Transformation|GetActorLocation) "0, 0, 0" 1.0 1.0 0.0 0 0 0)
      (goto _label Reset))))

(event Custom|Movement
  (AI|AIMoveTo self (.RandomLocation (Class|NavigationSystemV1|GetRandomPointinNavigableRadius (Transformation|GetActorLocation) 1e+03 0 0)) 0 5.0 false
    (:then
      (Utilities|FlowControl|Delay 5.0)
      (CallFunction|Movement))))

(event EventBeginPlay
  (Utilities|Time|SetTimerbyFunctionName 0 "Movement" 3.0))

(fn ConstructionScript
  (Transformation|AttachComponentToComponent (Variables|Default|GetPen) (Variables|Character|GetMesh) "Pen" "KeepRelative" "KeepRelative" "KeepRelative" true)
  (Transformation|AttachComponentToComponent (Variables|Default|GetClip) (Variables|Character|GetMesh) "Clip" "KeepRelative" "KeepRelative" "KeepRelative" true))